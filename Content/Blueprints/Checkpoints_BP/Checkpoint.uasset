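; Checkpoint actor that registers when a BP_HoverVehicle passes through it in the correct direction.
; When the vehicle leaves the box trigger, its forward vector is dotted against the Arrow component's direction, so only forward crossings count.
; A valid pass calls CallCheckpointCleared with the checkpoint number, hides the particle effect and trigger, and turns off overlap events so it fires once.
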(event OnComponentEndOverlap(BoxTrigger)
  (params (OverlappedComponent :type Primitive%20Component%20Object%20Reference) (OtherActor :type Actor%20Object%20Reference) (OtherComp :type Primitive%20Component%20Object%20Reference) (OtherBodyIndex :type Integer))
  ;[1 1 1] Checkpoint System
  (bind _asbp_hover_vehicle (Utilities|Casting|CastToBP_HoverVehicle OtherActor))
  (if (> (Math|Vector|DotProduct (Transformation|GetActorForwardVector _asbp_hover_vehicle) (Math|Rotator|GetRotationXVector (Transformation|GetWorldRotation (Variables|Default|GetArrow)))) 0.0)
    (Default|CallCheckpointCleared (Variables|Default|GetCheckpointNumber))
    (Development|SetHiddeninGame (Variables|Default|GetParticleSystem) true false)
    (Variables|/Script/Engine.PrimitiveComponent|SetbGenerateOverlapEvents (Variables|Default|GetBoxTrigger) false)))

(fn ConstructionScript)