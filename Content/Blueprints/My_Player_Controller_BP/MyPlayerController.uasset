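; Player controller for a hover vehicle race that tracks laps, race and lap times, and saved best times.
; Two timelines act as clocks, with the race clock starting after a delay, and feed text variables for the speed HUD.
; Lap updates compare times against the records and write improvements to a SaveGame slot.
; It also respawns the vehicle, shows the splash screen after the race, and resets records by key before the start.
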(event Custom|StartGameSetup
  ;[1 1 1] Starts the Game Setup - Checks if we have a game save and initialises the text
  (CallFunction|SaveGameCheck)
  (CallFunction|InitText))

(event Custom|Restart
  (bind _returnvalue (Game|GetPlayerController 0))
  (bind _my_player_controller_ref (Variables|Default|GetMy_Player_Controller_Ref))
  ;[1 1 1] Restart - If last checkpoint is complete then delya 6 seconds and load the main menu
  (if (Variables|Default|GetRaceComplete)
    (CallFunction|StopRaceTime)
    (Input|DisableInput (Variables|Default|GetVehicle%20Reference) _my_player_controller_ref)
    (Viewport|RemoveAllWidgets)
    (bind _returnvalue_2 (UserInterface|CreateWidget "/Game/UI/Splash_Screen_Widget/SplashScreen.SplashScreen_C" _my_player_controller_ref))
    (UserInterface|Viewport|AddtoViewport _returnvalue_2 0)
    (Input|SetInputModeUIOnly _returnvalue 0 "DoNotLock")
    (Variables|/Script/Engine.PlayerController|SetbShowMouseCursor _returnvalue true)))

(event Custom|UpdateLap
  ;[1 1 1] Update the Lap - Checks if race is complete, updates the actual lap and updates the lap time
  (if (Variables|Default|GetRaceComplete)
    _
    (else
      (bind _output_get (Variables|ValueVariables|SetActualLap (+ (Variables|ValueVariables|GetActualLap) 1)))
      (Variables|TextVariables|SetCurrentLapText (Utilities|Text|ToText(Integer) _output_get))))
  (CallFunction|LapTimeCheck))

(event Custom|RespawnVehicle
  ;[1 1 1] Respawn Vehicle - Gets the location of last checkpoint and spawns vehicle if flipped or fallen off map
  (bind _returnvalue (Game|SpawnActorfromClass "/Game/Blueprints/Main_Vehicle_BP/HoverFriction.BP_HoverVehicle_C" (Variables|Default|GetRespawnLocation) "Undefined" 0 0))
  (Pawn|Possess _returnvalue))

(event Custom|StartRaceTime
  (Utilities|FlowControl|Delay 9.5)
  ;[1 1 1] This controls the lap timer and updates the time goals
  (bind _time (Timeline|GameTime Play)
    (:Update
      (bind _output_get (Variables|ValueVariables|SetActualRaceTime _time))
      (Variables|TextVariables|SetRaceTimeText (Utilities|TimetoText _output_get))
      (CallFunction|UpdateGoals))))

(event Custom|StopRaceTime
  ;[1 1 1] This controls the lap timer and updates the time goals
  (bind _time (Timeline|GameTime Stop)
    (:Update
      (bind _output_get (Variables|ValueVariables|SetActualRaceTime _time))
      (Variables|TextVariables|SetRaceTimeText (Utilities|TimetoText _output_get))
      (CallFunction|UpdateGoals))))

(event Custom|StartLapTime
  ;[1 1 1] This controls the lap timer and updates the time goals
  (bind _time (Timeline|LapTime PlayFromStart)
    (:Update
      (Variables|ValueVariables|SetActualLapTime _time))))

(event Custom|StopLapTime
  ;[1 1 1] This controls the lap timer and updates the time goals
  (bind _time (Timeline|LapTime Stop)
    (:Update
      (Variables|ValueVariables|SetActualLapTime _time))))

(event EventBeginPlay
  ;[1 1 1] Event Begin Play - Gets the vehicles reference, Starts the Race Time and Lap Time
  (bind _asbp_hover_vehicle (Utilities|Casting|CastToBP_HoverVehicle (Game|Player|GetPlayerPawn 0)))
  (Variables|Default|SetVehicle%20Reference _asbp_hover_vehicle)
  (CallFunction|StartRaceTime)
  (CallFunction|StartLapTime))

(event Input|KeyboardEvents|0
  (params (Key :type Key%20Structure))
  ;[1 1 1] Resets to default times if race not started
  (:Pressed
    (if (not (Variables|Default|GetRaceStart))
      (Variables|ValueVariables|SetBestLapTime (Variables|ValueVariables|GetDefaultBestLapTime))
      (Variables|ValueVariables|SetBestRaceTime (Variables|ValueVariables|GetDefaultBestRaceTime))
      (CallFunction|SavetheGame)
      (CallFunction|InitText))))

(event Input|KeyboardEvents|9
  (params (Key :type Key%20Structure))
  (:Pressed
    (Variables|TextVariables|SetBestTimeText (Utilities|TimetoText (Variables|ValueVariables|GetBestLapTime)))
    (Variables|TextVariables|SetBestLapText (Utilities|TimetoText (Variables|ValueVariables|GetBestRaceTime)))))

(fn ConstructionScript)

(fn InitText
  ;[1 1 1] Values for SpeedHUD
  (Variables|TextVariables|SetCurrentLapText (Utilities|Text|ToText(Integer) (Variables|ValueVariables|GetActualLap)))
  (Variables|TextVariables|SetMaxLapText (Utilities|Text|ToText(Integer) (Variables|ValueVariables|GetMaxLaps)))
  (Variables|TextVariables|SetRaceTimeText (Utilities|TimetoText (Variables|ValueVariables|GetActualRaceTime)))
  (Variables|TextVariables|SetBestTimeText (Utilities|TimetoText (Variables|ValueVariables|GetActualLapTime)))
  (Variables|TextVariables|SetBestLapText (Utilities|TimetoText (Variables|ValueVariables|GetBestLapTime)))
  (Variables|TextVariables|SetBestTimeText (Utilities|TimetoText (Variables|ValueVariables|GetBestRaceTime))))

(fn SaveGameCheck
  ;[1 1 1] If game is saved then set the default time as the best lap and race time
  (bind _returnvalue (SaveGame|DoesSaveGameExist (Variables|Default|GetSaveSlot)))
  (if _returnvalue
    (CallFunction|LoadtheGame)
    (else
      (Variables|ValueVariables|SetBestLapTime (Variables|ValueVariables|GetDefaultBestLapTime))
      (Variables|ValueVariables|SetBestRaceTime (Variables|ValueVariables|GetDefaultBestRaceTime))
      (CallFunction|SavetheGame))))

(fn SavetheGame
  ;[1 1 1] Saving the game to a slot
  (bind _returnvalue (SaveGame|CreateSaveGameObject "/Game/Blueprints/Game_Save_BP/MySaveGame.MySaveGame_C"))
  (bind _output_get (Variables|Default|SetReferenceToSaveGame _returnvalue))
  (bind _asmy_save_game (Utilities|Casting|CastToMySaveGame _output_get))
  (Variables|/Game/Blueprints/Game_Save_BP/MySaveGame.MySaveGame_C|SetSavingBestLapTime _asmy_save_game (Variables|ValueVariables|GetBestLapTime))
  (Variables|/Game/Blueprints/Game_Save_BP/MySaveGame.MySaveGame_C|SetSavingBestRaceTime _asmy_save_game (Variables|ValueVariables|GetBestRaceTime))
  (SaveGame|SaveGametoSlot (Variables|Default|GetReferenceToSaveGame) (Variables|Default|GetSaveSlot)))

(fn LoadtheGame
  ;[1 1 1] Loads the saved game. Has best lap and race time saved
  (bind _returnvalue (SaveGame|LoadGamefromSlot (Variables|Default|GetSaveSlot)))
  (bind _asmy_save_game (Utilities|Casting|CastToMySaveGame _returnvalue))
  (Variables|ValueVariables|SetBestLapTime (Variables|/Game/Blueprints/Game_Save_BP/MySaveGame.MySaveGame_C|GetSavingBestLapTime _asmy_save_game))
  (Variables|ValueVariables|SetBestRaceTime (Variables|/Game/Blueprints/Game_Save_BP/MySaveGame.MySaveGame_C|GetSavingBestRaceTime _asmy_save_game)))

(fn LapTimeCheck
  ;[1 1 1] Checks the Lap Time
  (CallFunction|StopLapTime)
  (if (<= (Variables|ValueVariables|GetActualLapTime) (Variables|ValueVariables|GetBestLapTime))
    (bind _output_get (Variables|ValueVariables|SetBestLapTime (Variables|ValueVariables|GetActualLapTime)))
    (Variables|TextVariables|SetBestLapText (Utilities|TimetoText _output_get))
    (CallFunction|SavetheGame)
    (Variables|ValueVariables|SetActualLapTime 0.0)
    (else
      (Variables|ValueVariables|SetActualLapTime 0.0)))
  (if (Variables|Default|GetRaceComplete)
    (CallFunction|RaceTimeCheck)
    (else
      (CallFunction|StartLapTime))))

(fn RaceTimeCheck
  ;[1 1 1] Checks the Race Time and saves the time
  (if (<= (Variables|ValueVariables|GetActualRaceTime) (Variables|ValueVariables|GetBestRaceTime))
    (bind _output_get (Variables|ValueVariables|SetBestRaceTime (Variables|ValueVariables|GetActualRaceTime)))
    (Variables|TextVariables|SetBestTimeText (Utilities|TimetoText _output_get))
    (CallFunction|SavetheGame)))

(fn UpdateGoals)