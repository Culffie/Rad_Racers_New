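; Player-driven hover vehicle that waits for a countdown event, then follows track surfaces using interpolated throttle and steering.
; Each tick moves it forward, sphere-traces down to hold hover height and align to the surface normal, or drops it without a hit.
; Gravity volumes or Enter switch to zero-G rotation with held speed.
; Overlaps change health; death briefly hides it, while being stuck tipped over destroys it and requests a controller respawn.
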(event OnComponentBeginOverlap(HealthColl)
  (params (OverlappedComponent :type Primitive%20Component%20Object%20Reference) (OtherActor :type Actor%20Object%20Reference) (OtherComp :type Primitive%20Component%20Object%20Reference) (OtherBodyIndex :type Integer) (bFromSweep :type Boolean) (SweepResult :type Hit%20Result%20Structure%20%28by%20ref%29))
  ;[1 1 1] Damage & Health
  (Utilities|Casting|CastTo OtherActor)
  (if (< (Variables|Default|GetHealth) 100)
    (Variables|Default|SetHealth (+ (Variables|Default|GetHealth) 10))))

(event OnComponentBeginOverlap(DamageColl)
  (params (OverlappedComponent :type Primitive%20Component%20Object%20Reference) (OtherActor :type Actor%20Object%20Reference) (OtherComp :type Primitive%20Component%20Object%20Reference) (OtherBodyIndex :type Integer) (bFromSweep :type Boolean) (SweepResult :type Hit%20Result%20Structure%20%28by%20ref%29))
  ;[1 1 1] Damage & Health
  (Utilities|Casting|CastTo OtherActor)
  (if (> (Variables|Default|GetHealth) 0)
    (Variables|Default|SetHealth (- (Variables|Default|GetHealth) 10))))

(event OnComponentBeginOverlap(GravColl)
  (params (OverlappedComponent :type Primitive%20Component%20Object%20Reference) (OtherActor :type Actor%20Object%20Reference) (OtherComp :type Primitive%20Component%20Object%20Reference) (OtherBodyIndex :type Integer) (bFromSweep :type Boolean) (SweepResult :type Hit%20Result%20Structure%20%28by%20ref%29))
  (bind _cube (Variables|Default|GetCube))
  ;[1 1 1] Gravity Toggle
  (Utilities|Casting|CastTo OtherActor)
  (Variables|Default|SetGravity false)
  (Development|PrintString "Gravity Off")
  (Physics|SetSimulatePhysics _cube true)
  (Physics|SetEnableGravity _cube false))

(event OnComponentEndOverlap(GravColl)
  (params (OverlappedComponent :type Primitive%20Component%20Object%20Reference) (OtherActor :type Actor%20Object%20Reference) (OtherComp :type Primitive%20Component%20Object%20Reference) (OtherBodyIndex :type Integer))
  ;[1 1 1] Gravity Toggle
  (Utilities|Casting|CastTo OtherActor)
  (Variables|Default|SetGravity true)
  (Development|PrintString "Gravity On")
  (Physics|SetSimulatePhysics (Variables|Default|GetCube) false))

(event OnComponentBeginOverlap(WallColl)
  (params (OverlappedComponent :type Primitive%20Component%20Object%20Reference) (OtherActor :type Actor%20Object%20Reference) (OtherComp :type Primitive%20Component%20Object%20Reference) (OtherBodyIndex :type Integer) (bFromSweep :type Boolean) (SweepResult :type Hit%20Result%20Structure%20%28by%20ref%29))
  ;[1 1 1] Damage & Health
  (Utilities|Casting|CastTo OtherActor)
  (if (> (Variables|Default|GetHealth) 0)
    (Variables|Default|SetHealth (- (Variables|Default|GetHealth) 5))))

(event Custom|Start%20Camera%20Location
  (bind _deltas (Variables|Default|GetdeltaS))
  (bind _returnvalue (Math|Vector|Normalize _deltas))
  ;[1 1 1] Camera Location
  (Transformation|SetRelativeLocation (Variables|Default|GetSpringArm) (Math|Interpolation|VInterpTo (Variables|/Script/Engine.SceneComponent|GetRelativeLocation (Variables|Default|GetSpringArm)) (Math|Vector|MakeVector -4.64904 (+ 0.0 -4.0 (* (* (.yaw (Math|Transform|InverseTransformRotation (Transformation|GetActorTransform) (Math|Rotator|FindLookatRotation (Math|Vector|MakeVector 0.0 0.0 0.0) (/ (+ (Math|Vector|MakeVector (* (.x _returnvalue) 1e+02) (* (.y _returnvalue) 1e+02) (* (.z _returnvalue) 2e+02)) (* (Math|Vector|GetForwardVector (Variables|Default|GetCube)) 4.0)) 1.0)))) -6.0 -0.03) -3e+01 (/ (Variables|Default|GetCurrentSpeed) (Variables|Default|GetMaxSpeed)))) 11.933249) (Utilities|Time|GetWorldDeltaSeconds) 1.0) true false))

(event Custom|Line%20trace%20safety
  (bind _returnvalue (Utilities|Time|GetWorldDeltaSeconds))
  (bind _returnvalue_2 (Math|Rotator|MakeRotator 0.0 0.0 0.0))
  (bind _returnvalue_3 (Transformation|GetActorRotation))
  (bind _cube (Variables|Default|GetCube))
  (bind _returnvalue_4 (Transformation|GetWorldLocation _cube))
  (bind _returnvalue_5 (Math|Interpolation|RInterpTo _returnvalue_3 _returnvalue_2 _returnvalue 6.0))
  ;[1 1 1] Track Hover and Alignment
  (if (Variables|Default|GetGravity)
    (bind (_outhit _returnvalue_6) (Collision|SphereTraceByChannel _returnvalue_4 (+ (* (Math|Vector|GetUpVector _cube) -4e+02) _returnvalue_4) 6e+01 "TraceTypeQuery1" false 0 "ForOneFrame"))
    (if _returnvalue_6
      (Transformation|SetActorRotation (Math|Interpolation|RInterpTo (Transformation|GetActorRotation) (Math|Rotator|MakeRotfromZX (.ImpactNormal (Collision|BreakHitResult _outhit)) (Transformation|GetActorForwardVector)) _returnvalue 6.0))
      (Transformation|SetActorLocation (+ (.ImpactPoint (Collision|BreakHitResult _outhit)) (* (.ImpactNormal (Collision|BreakHitResult _outhit)) 1.5e+02)) false false)
      (Utilities|FlowControl|DoOnce true :!label _label
        (:Completed
          (Class|PlayerController|ClientPlayCameraShake (Game|GetPlayerController 0) "/Script/Engine.CameraShake" 0.7 "CameraLocal" "0, 0, 0")))
      (else
        (Transformation|AddActorWorldOffset "0, 0,-60.000000")
        (Transformation|SetActorRotation (Math|Rotator|MakeRotator (.roll _returnvalue_5) (.pitch _returnvalue_5) (.Yaw (Math|Rotator|BreakRotator _returnvalue_3))))
        (goto _label Reset)))))

(event Custom|StartHover_1
  ;[1 1 1] Countdown Interface
  (Actor|Tick|SetActorTickEnabled true))

(event EventTick
  (params (DeltaSeconds :type Float%20%28single-precision%29))
  (bind _cube (Variables|Default|GetCube))
  (bind _cube_2 (Variables|Default|GetCube))
  ;[1 1 1] Tick - Move Forward/Backward
  (Utilities|FlowControl|Sequence
    (:then_0
      (if (Variables|Default|GetGravity)
        (bind _output_get (Variables|Default|SetCurrentSpeed (Math|Interpolation|FInterpTo (Variables|Default|GetCurrentSpeed) (Variables|Default|GetDesiredSpeed) (Utilities|Time|GetWorldDeltaSeconds) (/ (Variables|Default|GetAccelerationInterp) 2.0))))
        (Transformation|AddActorLocalOffset (Math|Vector|MakeVector _output_get 0.0 0.0) true false)
        (CallFunction|LineTraceSafety)
        ;[1 1 1] Death & Respawn
        (if (<= (Variables|Default|GetHealth) 0)
          (Input|DisableInput 0)
          (Collision|SetCollisionEnabled _cube_2 "NoCollision")
          (Rendering|SetVisibility _cube_2 false false)
          (Variables|Default|SetDesiredSpeed 0.0)
          (Variables|Default|SetCurrentSpeed 0.0)
          (Utilities|FlowControl|Delay 2.0)
          (Variables|Default|SetHealth 100)
          (Input|EnableInput 0)
          (Rendering|SetVisibility _cube true false)
          (Utilities|FlowControl|Delay 2.0)
          (Collision|SetCollisionEnabled _cube "QueryAndPhysics"))
        (else
          (bind _output_get_2 (Variables|Default|SetCurrentSpeed (Variables|Default|GetCurrentSpeed)))
          (Transformation|AddActorLocalOffset (Math|Vector|MakeVector _output_get_2 0.0 0.0) true false)
          (CallFunction|LineTraceSafety))))
    (:then_1
      (bind _playerisstuck (CallFunction|RespawnCheck))
      (if _playerisstuck
        (Utilities|FlowControl|Delay 4.0)
        (bind _playerisstuck_2 (CallFunction|RespawnCheck))
        (if _playerisstuck_2
          (Actor|DestroyActor))))))

(event EventBeginPlay
  ;[1 1 1] Countdown Interface
  (Actor|Tick|SetActorTickEnabled false)
  (bind _asmy_player_controller (Utilities|Casting|CastTo (Game|GetPlayerController 0)))
  (bind _output_get (Variables|Default|SetController%20Reference 0 _asmy_player_controller))
  (Variables|Default|SetRespawnLocation _output_get (Transformation|GetActorTransform))
  (Variables|Default|SetHealth 100))

(event EventDestroyed
  (CallFunction|RespawnVehicle (.Controller%20Reference (Variables|Default|GetController%20Reference))))

(event Collision|EventHit
  (params (MyComp :type Primitive%20Component%20Object%20Reference) (Other :type Actor%20Object%20Reference) (OtherComp :type Primitive%20Component%20Object%20Reference) (bSelfMoved :type Boolean) (HitLocation :type Vector :default "0, 0, 0") (HitNormal :type Vector :default "0, 0, 0") (NormalImpulse :type Vector :default "0, 0, 0") (Hit :type Hit%20Result%20Structure%20%28by%20ref%29))
  ;[1 1 1] Friction
  (Utilities|Casting|CastTo Other)
  (Variables|Default|SetMaxSpeed 3e+02)
  (Utilities|FlowControl|RetriggerableDelay 3.0)
  (Variables|Default|SetMaxSpeed 2.5e+02))

(event Input|AxisEvents|InputAxisThrottle/Pitch
  (params (AxisValue :type Float%20%28single-precision%29))
  ;[1 1 1] Throttle
  (if (Variables|Default|GetGravity)
    (if (> AxisValue 0.0)
      (Variables|Default|SetDesiredSpeed (Math|Interpolation|FInterpTo (Variables|Default|GetDesiredSpeed) (Variables|Default|GetMaxSpeed) (Utilities|Time|GetWorldDeltaSeconds) (Variables|Default|GetAccelerationInterp)))
      (elif (< AxisValue 0.0)
        (Variables|Default|SetDesiredSpeed (Math|Interpolation|FInterpTo (Variables|Default|GetDesiredSpeed) (* (/ (Variables|Default|GetMaxSpeed) 2.0) -1.0) (Utilities|Time|GetWorldDeltaSeconds) (Variables|Default|GetAccelerationInterp)))
        (elif (== 0.0 0.0)
          (Variables|Default|SetDesiredSpeed (Math|Interpolation|FInterpTo (Variables|Default|GetDesiredSpeed) 0.0 (Utilities|Time|GetWorldDeltaSeconds) 0.0)))))))

(event Input|AxisEvents|InputAxisYaw
  (params (AxisValue :type Float%20%28single-precision%29))
  ;[1 1 1] Yaw and Pitch
  (if (Variables|Default|GetGravity)
    (if (!= AxisValue 0.0)
      (Transformation|AddActorLocalRotation (Math|Rotator|MakeRotator AxisValue 0.0 AxisValue) false false))))

(event Input|AxisEvents|InputAxisThrottle/Pitch
  (params (AxisValue :type Float%20%28single-precision%29))
  ;[1 1 1] Zero G Flight
  (if (not (Variables|Default|GetGravity))
    (Transformation|AddActorLocalRotation (Math|Rotator|MakeRotator 0.0 (Math|Interpolation|FInterpTo AxisValue 1e+01 (Utilities|Time|GetWorldDeltaSeconds) 0.5) 0.0) false false)))

(event Input|AxisEvents|InputAxisYaw
  (params (AxisValue :type Float%20%28single-precision%29))
  ;[1 1 1] Zero G Flight
  (if (not (Variables|Default|GetGravity))
    (Transformation|AddActorLocalRotation (Math|Rotator|MakeRotator (Math|Interpolation|FInterpTo AxisValue 1e+01 (Utilities|Time|GetWorldDeltaSeconds) 0.5) 0.0 0.0) false false)))

(event Input|KeyboardEvents|SpaceBar
  (params (Key :type Key%20Structure))
  ;[1 1 1] Health Test
  (:Pressed
    (if (> (Variables|Default|GetHealth) 0)
      (Variables|Default|SetHealth (- (Variables|Default|GetHealth) 10))
      (else
        (Development|PrintString "Dead")))))

(event Input|KeyboardEvents|P
  (params (Key :type Key%20Structure))
  (bind _returnvalue (Transformation|GetActorLocation))
  ;[1 1 1] Death
  (:Pressed
    (bind _output_get (Variables|Default|SetDeathX (.x _returnvalue)))
    (bind _output_get_2 (Variables|Default|SetDeathY (.y _returnvalue)))
    (bind _output_get_3 (Variables|Default|SetDeathZ (.z _returnvalue)))
    (bind _output_get_4 (Variables|Default|SetDeathArea (+ _output_get_2 1e+04)))
    (Transformation|SetActorLocation (Math|Vector|MakeVector _output_get _output_get_4 _output_get_3) false false)
    (Utilities|FlowControl|Delay 2.0)
    (Transformation|SetActorLocation (Math|Vector|MakeVector _output_get _output_get_2 _output_get_3) false true)
    (Variables|Default|SetHealth 100)))

(event Input|KeyboardEvents|F
  (params (Key :type Key%20Structure))
  (:Pressed
    (if (Class|PrimitiveComponent|IsOverlappingComponent (Variables|Default|GetFricColl))
      _)))

(event Input|KeyboardEvents|Enter
  (params (Key :type Key%20Structure))
  (bind _cube (Variables|Default|GetCube))
  ;[1 1 1] Gravity Toggle
  (:Pressed
    (Variables|Default|SetGravity false)
    (Development|PrintString "Gravity Off")
    (Physics|SetSimulatePhysics _cube true)
    (Physics|SetEnableGravity _cube false))
  (:Released
    (Variables|Default|SetGravity true)
    (Development|PrintString "Gravity On")
    (Physics|SetSimulatePhysics _cube false)))

(fn ConstructionScript)

(fn SplitAxis
  (params (Value :type Float%20%28single-precision%29))
  (return (Math|Float|Clamp(Float) Value) (Math|Float|Clamp(Float) (- 0.0 Value))))

(fn RespawnCheck
  ;[1 1 1] Checks to see if player is not moving and upside down
  (if (and (< (Math|Vector|DotProduct (Transformation|GetActorUpVector) "0, 0,1.000000") 0.5) (< (Variables|Default|GetCurrentSpeed) 0.5))
    (Variables|Default|SetStuck? true)
    (else
      (Variables|Default|SetStuck? false)))
  (return (Variables|Default|GetStuck?)))