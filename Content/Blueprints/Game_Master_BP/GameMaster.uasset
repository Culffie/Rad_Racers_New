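; Game master actor that starts the hover actors and ranks them by their progress along a reference spline.
; BeginPlay plays a sound, waits briefly, then sends StartHoverMessage to every HoverInterface actor.
; Each Tick maps every actor's spline distance to that actor, sorts the distances in reverse and rebuilds ActorList in rank order.
; A helper finds that distance by interpolating between spline points using the closest input key.
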(event EventBeginPlay
  (Audio|PlaySound2D 0 1.0 1.0 12.2 0 0)
  (Utilities|FlowControl|Delay 5.0)
  (bind _outactors (Actor|GetAllActorswithInterface "/Game/Blueprints/Main_Vehicle_BP/HoverInterface.HoverInterface_C"))
  (for _array_element _outactors
    (Class|HoverInterface|StartHover(Message) _array_element)))

(event Collision|EventActorBeginOverlap
  (params (OtherActor :type Actor%20Object%20Reference)))

(event EventTick
  (params (DeltaSeconds :type Float%20%28single-precision%29))
  (Utilities|Array|Clear (Variables|Default|GetSorted_List))
  (Utilities|Array|Clear (Variables|Default|GetActorList))
  (Utilities|Map|Clear (Variables|Default|GetRanking))
  ;[1 1 1] Get all actor which use Hover Interface
  (bind _outactors (Actor|GetAllActorswithInterface "/Game/Blueprints/Main_Vehicle_BP/HoverInterface.HoverInterface_C"))
  (for _array_element _outactors
    (Utilities|Map|Add (Variables|Default|GetRanking) (CallFunction|FindDistanceAlongSplineClosesttoWorldLocation (Transformation|GetActorLocation _array_element) (Variables|Default|GetSplineReference)) _array_element)
    (Utilities|Array|Add (Variables|Default|GetSorted_List) (CallFunction|FindDistanceAlongSplineClosesttoWorldLocation (Transformation|GetActorLocation _array_element) (Variables|Default|GetSplineReference))))
  ;[1 1 1] Sorting the array list and checking each array element in ranking
  (Variables|Default|SetSorted_List (Class|LowEntryExtendedStandardLibrary|SortFloatArray (Variables|Default|GetSorted_List) true))
  (for _array_element_2 (Variables|Default|GetSorted_List)
    ;[1 1 1] Actor list sorts each ranking in order e.g 0-10
    (Utilities|Array|Add (Variables|Default|GetActorList) (.Value (Utilities|Map|Find (Variables|Default|GetRanking) _array_element_2)))))

(fn ConstructionScript)

(fn FindDistanceAlongSplineClosesttoWorldLocation
  (params (Location :type Vector) (Spline :type Track%20Object%20Reference))
  (bind _usefulspline (Variables|/Game/Blueprints/AIFollow_Spline/Track.Track_C|GetUsefulSpline Spline))
  (bind _returnvalue (Class|SplineComponent|FindInputKeyClosesttoWorldLocation _usefulspline Location))
  (bind _returnvalue_2 (Math|Float|Truncate _returnvalue))
  (bind _returnvalue_3 (Spline|GetDistanceAlongSplineatSplinePoint _usefulspline _returnvalue_2))
  (return (+ _returnvalue_3 (* (- (Spline|GetDistanceAlongSplineatSplinePoint _usefulspline (Math|Float|Truncate (+ _returnvalue 1.0))) _returnvalue_3) (- _returnvalue (Math|Conversions|ToFloat(Integer) _returnvalue_2))))))