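; Track-building spline actor that lays repeated meshes along an editable, optionally closed spline in its construction script.
; It divides the spline by section length, adding a collision-enabled spline mesh per section with position and tangents sampled by distance.
; Roll and cross-section scale come from spline points indexed by section number rather than distance, so they align only when points match section boundaries.
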(event EventBeginPlay)

(event Collision|EventActorBeginOverlap
  (params (OtherActor :type Actor%20Object%20Reference)))

(event EventTick
  (params (DeltaSeconds :type Float%20%28single-precision%29)))

(fn ConstructionScript
  (Spline|SetClosedLoop (Variables|Default|GetTrack_Spline) (Variables|Default|GetClosed%20Loop?) true)
  (for _index (range 0 (Math|Float|Truncate (/ (Spline|GetSplineLength (Variables|Default|GetTrack_Spline)) (Variables|Default|GetSectionLength))))
    (LocalVariables|SetStartPoint _index)
    (LocalVariables|SetEndPoint (+ _index 1))
    (bind _returnvalue (AddComponent|AddSplineMeshComponent false))
    (SplineMesh|SetForwardAxis _returnvalue "X" true)
    (Collision|SetCollisionEnabled _returnvalue "QueryAndPhysics")
    (bind _output_get (LocalVariables|SetSpline%20Mesh _returnvalue))
    (Components|StaticMesh|SetStaticMesh _output_get (Variables|Default|GetTrack%20Mesh))
    (SplineMesh|SetStartandEnd (LocalVariables|GetSpline%20Mesh) (Spline|GetLocationatDistanceAlongSpline (Variables|Default|GetTrack_Spline) (* _index (Variables|Default|GetSectionLength)) "Local") (Spline|GetTangentatDistanceAlongSpline (Variables|Default|GetTrack_Spline) (* _index (Variables|Default|GetSectionLength)) "Local") (Spline|GetLocationatDistanceAlongSpline (Variables|Default|GetTrack_Spline) (* (+ _index 1) (Variables|Default|GetSectionLength)) "Local") (Spline|GetTangentatDistanceAlongSpline (Variables|Default|GetTrack_Spline) (* (+ _index 1) (Variables|Default|GetSectionLength)) "Local") true :!class /Script/Engine.SplineMeshComponent)
    (Class|SplineMeshComponent|SetStartRoll (LocalVariables|GetSpline%20Mesh) (Math|Trig|DegreesToRadians (Spline|GetRollatSplinePoint (Variables|Default|GetTrack_Spline) (LocalVariables|GetStartPoint) "Local")) true)
    (Class|SplineMeshComponent|SetEndRoll (LocalVariables|GetSpline%20Mesh) (Math|Trig|DegreesToRadians (Spline|GetRollatSplinePoint (Variables|Default|GetTrack_Spline) (LocalVariables|GetEndPoint) "Local")) true)
    (SplineMesh|SetStartScale (LocalVariables|GetSpline%20Mesh) (Math|Vector2D|MakeVector2D (.y (Spline|GetScaleatSplinePoint (Variables|Default|GetTrack_Spline) (LocalVariables|GetStartPoint))) (.z (Spline|GetScaleatSplinePoint (Variables|Default|GetTrack_Spline) (LocalVariables|GetStartPoint)))) true :!class /Script/Engine.SplineMeshComponent)
    (SplineMesh|SetEndScale (LocalVariables|GetSpline%20Mesh) (Math|Vector2D|MakeVector2D (.y (Spline|GetScaleatSplinePoint (Variables|Default|GetTrack_Spline) (LocalVariables|GetEndPoint))) (.z (Spline|GetScaleatSplinePoint (Variables|Default|GetTrack_Spline) (LocalVariables|GetEndPoint)))) true :!class /Script/Engine.SplineMeshComponent)))