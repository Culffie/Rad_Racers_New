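; Spline-driven road actor that builds curvy track pieces along an editable spline in the construction script.
; It divides the spline length by a base piece length and adds a spline mesh component per segment, set from sampled locations and tangents.
; Spline scale times Width and Height shapes each end, and world-space roll divided by a constant sets banking.
; A flag toggles collision on the pieces.
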(fn ConstructionScript
  (bind _returnvalue (Math|Float|MakeLiteralFloat 5e+01))
  (bind _base_length_multiplier (Variables|GenerationData|GetBase%20length%20multiplier))
  (bind _userspline (Variables|Default|GetUserSpline))
  (bind _userspline_2 (Variables|Default|GetUserSpline))
  (Variables|Default|SetNumber%20of%20track%20pieces (Math|Float|Truncate (/ (Spline|GetSplineLength (Variables|Default|GetUserSpline)) (Variables|GenerationData|GetBase%20length%20multiplier))))
  (for _index (range 0 (- (Variables|Default|GetNumber%20of%20track%20pieces) 0))
    (bind _output_get (Variables|Default|SetCurrent%20index _index))
    ;[1 1 1] Insert Mesh
    (bind _returnvalue_2 (AddComponent|AddSplineMeshComponent false))
    (SplineMesh|SetStartandEnd _returnvalue_2 (.Location (Utilities|GetLocationandTangentatDistanceAlongSpline _userspline_2 (* _output_get _base_length_multiplier) true)) (.Tangent (Utilities|GetLocationandTangentatDistanceAlongSpline _userspline_2 (* _output_get _base_length_multiplier) true)) (.Location (Utilities|GetLocationandTangentatDistanceAlongSpline _userspline_2 (* (+ _output_get 1) _base_length_multiplier) true)) (.Tangent (Utilities|GetLocationandTangentatDistanceAlongSpline _userspline_2 (* (+ _output_get 1) _base_length_multiplier) true)) true :!class /Script/Engine.SplineMeshComponent)
    (SplineMesh|SetStartScale _returnvalue_2 (Math|Vector2D|MakeVector2D (* (Variables|GenerationData|GetWidth) (.y (Class|SplineComponent|GetScaleatDistanceAlongSpline _userspline_2 (* _output_get _base_length_multiplier)))) (* (Variables|GenerationData|GetHeight) (.z (Class|SplineComponent|GetScaleatDistanceAlongSpline _userspline_2 (* _output_get _base_length_multiplier))))) true :!class /Script/Engine.SplineMeshComponent)
    (SplineMesh|SetEndScale _returnvalue_2 (Math|Vector2D|MakeVector2D (* (Variables|GenerationData|GetWidth) (.y (Class|SplineComponent|GetScaleatDistanceAlongSpline _userspline (* (+ _output_get 1) _base_length_multiplier)))) (* (Variables|GenerationData|GetHeight) (.z (Class|SplineComponent|GetScaleatDistanceAlongSpline _userspline (* (+ _output_get 1) _base_length_multiplier))))) true :!class /Script/Engine.SplineMeshComponent)
    (Class|SplineMeshComponent|SetStartRoll _returnvalue_2 (/ (CallFunction|GetRelativeRollatDistanceAlongSpline _userspline_2 (* _output_get _base_length_multiplier) "0, 0, 0") _returnvalue) true)
    (Class|SplineMeshComponent|SetEndRoll _returnvalue_2 (/ (CallFunction|GetRelativeRollatDistanceAlongSpline _userspline (* (+ _output_get 1) _base_length_multiplier) "0, 0, 0") _returnvalue) true)
    (Collision|SetCollisionEnabled _returnvalue_2 (select (Variables|Default|GetCalculate%20Collision) "QueryAndPhysics" "NoCollision"))))

(fn GetRelativeRollatDistanceAlongSpline
  (params (Spline :type Spline%20Component%20Object%20Reference) (Distance :type Float%20%28single-precision%29) (relative%20to :type Rotator))
  (return (.roll (Spline|GetRotationatDistanceAlongSpline Spline Distance "World"))))